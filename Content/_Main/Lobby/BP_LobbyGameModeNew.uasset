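; Lobby game mode that handles players joining a multiplayer lobby.
; On PostLogin it records the player, caches all PlayerStart actors, and reads server name and player count from the game instance.
; It then has the player's controller run initial setup, build the lobby menu, and show default map settings through message calls.
; It finally calls SpawnPlayer, which is an empty event here.
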(event Custom|Spawn%20Player
  (params (Player :type Player%20Controller%20Object%20Reference)))

(event EventPostLogin
  (params (NewPlayer :type Player%20Controller%20Object%20Reference))
  (bind _output_get (Variables|Default|Setconnected%20player NewPlayer))
  (Utilities|Array|AddUnique (Variables|Default|Getplayers) _output_get)
  (bind _outactors (Actor|GetAllActorsOfClass "/Script/Engine.PlayerStart"))
  (Variables|Default|SetSpawnPoint _outactors)
  (bind _game_instance (Class|BpiGameinstance|SteamGameInstanceRef(Message) (Game|GetGameInstance)))
  (Variables|Default|SetServer%20Name? (Variables|/Game/_Main/Steamgameinstance.Steamgameinstance_C|GetServer%20Name? _game_instance))
  (Variables|Default|SetNumber%20Of%20Players? (Variables|/Game/_Main/Steamgameinstance.Steamgameinstance_C|GetNumber%20Of%20Players? _game_instance))
  (bind _lobby_pc (Class|BPI-LobbyPC|LobbyPCRef(Message) (Variables|Default|Getconnected%20player)))
  (Default|InitialSetup _lobby_pc)
  (Default|LobbyMenuSetup _lobby_pc (Variables|Default|GetServer%20Name?))
  (Default|UpdateLobbySettings _lobby_pc (Variables|Default|GetDefault%20map%20image) (Variables|Default|GetDefault%20Map%20Name) (Variables|Default|GetDefault%20Map%20Time))
  (CallFunction|SpawnPlayer (Variables|Default|Getconnected%20player)))

(fn ConstructionScript)